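; Collectible crystal Blueprint that flies to the player and vanishes when its trigger is overlapped.
; Overlap plays the CrystalMovement timeline, which each update lerps the actor from its current location toward player pawn 0 and fades the point light's intensity to zero.
; The actor destroys itself when the timeline finishes.
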(event OnComponentBeginOverlap(trigger)
  (params (OverlappedComponent :type Primitive%20Component%20Object%20Reference) (OtherActor :type Actor%20Object%20Reference) (OtherComp :type Primitive%20Component%20Object%20Reference) (OtherBodyIndex :type Integer) (bFromSweep :type Boolean) (SweepResult :type Hit%20Result%20Structure%20%28by%20ref%29))
  (bind (_direction _crystal_movement _crystal_light) (Timeline|Crystal%20movement Play)
    (:Update
      (Transformation|SetActorLocation (Math|Vector|Lerp(Vector) (Transformation|GetActorLocation) (Transformation|GetActorLocation (Game|Player|GetPlayerPawn 0)) _crystal_movement) false false)
      (Rendering|Components|Light|SetIntensity (Variables|Default|GetPointLight) (Math|Float|Lerp (Variables|Default|Getcrystal%20light%20intensity) 0.0 _crystal_light)))
    (:Finished
      (Actor|DestroyActor))))

(fn ConstructionScript)